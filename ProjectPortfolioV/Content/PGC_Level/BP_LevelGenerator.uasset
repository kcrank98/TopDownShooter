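; BP_LevelGenerator procedurally assembles a level on BeginPlay from randomly chosen room actors, starting with a root room and entrance plug.
; Each step removes a random open exit and spawns a random LevelList room there.
; Rooms whose overlap boxes hit anything are destroyed and generation recurses on another exit; accepted rooms add their exits and enemy spawn points.
; When the room count runs out, remaining exits are plugged.
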(event Custom|SpawnRootLevel
  ;[0 1 0.09089] Spawn Root Level
  (bind _returnvalue (Game|SpawnActorfromClass "/Game/PGC_Level/BP_LevelToGenerate1.BP_LevelToGenerate1_C" (Transformation|GetWorldTransform (Variables|Default|GetDefaultSceneRoot)) "AlwaysSpawn" "MultiplyWithRoot" 0 0))
  (Utilities|Array|AppendArray (Variables|Default|GetExitsList) (Components|GetChildrenComponents (Variables|/Game/PGC_Level/BP_MasterLevel.BP_MasterLevel_C|GetExitsFolder _returnvalue) false))
  (Utilities|Array|AppendArray (Variables|Default|GetSpawnList) (Components|GetChildrenComponents (Variables|/Game/PGC_Level/BP_MasterLevel.BP_MasterLevel_C|GetEnemySpawnFolder _returnvalue) false))
  (Variables|Default|SetNumberOfRooms (- (Variables|Default|GetNumberOfRooms) 1))
  (Game|SpawnActorfromClass "/Game/PGC_Level/BP_EntrancePlug.BP_EntrancePlug_C" (Transformation|GetWorldTransform (Components|GetChildComponent (Variables|/Game/PGC_Level/BP_MasterLevel.BP_MasterLevel_C|GetEntranceFolder _returnvalue) 0)) "Undefined" "MultiplyWithRoot" 0 0))

(event Custom|SpawnNextLevel
  (bind _exitslist (Variables|Default|GetExitsList))
  ;[0 1 0.09089] Spawn Next Level
  (bind _output_get (Variables|Default|SetSelectedExit (.OutItem (Utilities|Array|Random _exitslist))))
  (Utilities|Array|RemoveItem _exitslist _output_get)
  (bind _returnvalue (Game|SpawnActorfromClass (.OutItem (Utilities|Array|Random (Variables|Default|GetLevelList))) (Transformation|GetWorldTransform _output_get) "AlwaysSpawn" "MultiplyWithRoot" 0 0))
  (bind _asbp_master_level (Utilities|Casting|CastToBP_MasterLevel _returnvalue))
  (Variables|Default|SetCurrLevel _asbp_master_level)
  (CallFunction|CheckforOverlap))

(event Custom|CheckOverlapping
  ;[0 1 0.09089] Check For Overlapping Levels
  (for _array_element (Components|GetChildrenComponents (Variables|/Game/PGC_Level/BP_MasterLevel.BP_MasterLevel_C|GetOverlapFolder (Variables|Default|GetCurrLevel)) false)
    (bind _asbox_collision (Utilities|Casting|CastToBoxComponent _array_element))
    (Utilities|Array|AppendArray (Variables|Default|GetOverlapList) (Class|PrimitiveComponent|GetOverlappingComponents _asbox_collision))))

(event Custom|CheckForOverlap
  (bind _overlaplist (Variables|Default|GetOverlapList))
  (bind _currlevel (Variables|Default|GetCurrLevel))
  ;[0 1 0.09089] If No Overlapping Spawn Next Level
  (CallFunction|CheckOverlapping)
  (if (Utilities|Array|IsNotEmpty _overlaplist)
    (Utilities|Array|Clear _overlaplist)
    (Actor|DestroyActor (Variables|Default|GetCurrLevel))
    (CallFunction|SpawnNextLevel)
    (else
      (Utilities|Array|Clear _overlaplist)
      (bind _output_get (Variables|Default|SetNumberOfRooms (- (Variables|Default|GetNumberOfRooms) 1)))
      (Utilities|Array|AppendArray (Variables|Default|GetExitsList) (Components|GetChildrenComponents (Variables|/Game/PGC_Level/BP_MasterLevel.BP_MasterLevel_C|GetExitsFolder _currlevel) false))
      (Utilities|Array|AppendArray (Variables|Default|GetSpawnList) (Components|GetChildrenComponents (Variables|/Game/PGC_Level/BP_MasterLevel.BP_MasterLevel_C|GetEnemySpawnFolder _currlevel) false))
      (if (> _output_get 0)
        (CallFunction|SpawnNextLevel)
        (else
          (CallFunction|CloseExits))))))

(event Custom|CloseExits
  (bind _exitslist (Variables|Default|GetExitsList))
  ;[0 1 0.09089] Plug Unused Exits
  (for _array_element _exitslist
    (Game|SpawnActorfromClass "/Game/PGC_Level/BP_ExitPlug.BP_ExitPlug_C" (Transformation|GetWorldTransform _array_element) "AlwaysSpawn" "MultiplyWithRoot" 0 0))
  (Utilities|Array|Clear _exitslist))

(event EventBeginPlay
  ;[1 1 1] Begin Play
  (CallFunction|SpawnRootLevel)
  (CallFunction|SpawnNextLevel))

(fn ConstructionScript)