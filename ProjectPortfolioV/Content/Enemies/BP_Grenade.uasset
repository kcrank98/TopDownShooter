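; BP_Grenade is an enemy grenade that launches forward and up on spawn, then detonates on a timer.
; Detonation distance-checks only player 0 against BlastRadius, applying damage if the owner casts to Controller.
; Damage scales by distance clamped to 0–1, so it is effectively flat rather than falling off.
; Debug prints report outcomes before destruction, delayed on a miss; the construction script only scales SphereCollider.
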(event EventBeginPlay
  (bind _returnvalue (Game|GetPlayerCharacter 0))
  (bind _self self)
  (bind _returnvalue_2 (Transformation|GetActorLocation _returnvalue))
  (bind _returnvalue_3 (Transformation|GetActorLocation _self))
  (bind _returnvalue_4 (Math|Vector|Distance(Vector) _returnvalue_2 _returnvalue_3))
  (|CallParentFunction)
  (Game|Components|ProjectileMovement|SetVelocityinLocalSpace (Variables|Default|GetProjectileMovement) "10.000000,0.000000,10.000000")
  (Utilities|FlowControl|Delay (Variables|Default|GetDetonateTimer))
  (if (<= _returnvalue_4 (Variables|Default|GetBlastRadius))
    (bind _ascontroller (Utilities|Casting|CastToController (Components|GetOwner))
      (:then
        (bind _returnvalue_5 (Game|Damage|ApplyDamage _returnvalue (* (Variables|Default|GetDamageAmount) (Math|Float|Clamp(Float) _returnvalue_4)) _ascontroller self))
        (Development|PrintString (Utilities|String|ToString(Float) _returnvalue_5))
        (Actor|DestroyActor))
      (:CastFailed
        (Development|PrintString "grenade failed to get Owner Controller")
        (Actor|DestroyActor)))
    (else
      (Development|PrintString "did not hit player")
      (Utilities|FlowControl|Delay 2.0)
      (Actor|DestroyActor))))

(event Collision|EventActorBeginOverlap
  (params (OtherActor :type Actor%20Object%20Reference)))

(event EventTick
  (params (DeltaSeconds :type Float%20%28single-precision%29)))

(fn ConstructionScript
  (Transformation|SetWorldScale3D (Variables|Default|GetSphereCollider) (Variables|Default|GetSphereSize)))