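; Short-lived grenade explosion actor that pushes nearby physics objects and damages actors it overlaps.
; The construction script scales the collision sphere by Scale and binds its begin-overlap event.
; BeginPlay fires the radial force impulse, sets a brief lifespan and caches the owner as a Controller.
; HandleOverlap applies Damage to each overlapping actor, crediting that controller as instigator and the explosion as causer.
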(event EventBeginPlay
  (Class|RadialForceComponent|FireImpulse (Variables|Default|GetRadialForce))
  (Actor|SetLifeSpan 3.0)
  (bind _ascontroller (Utilities|Casting|CastToController (Components|GetOwner)))
  (Variables|Default|SetOwnerController _ascontroller))

(fn ConstructionScript
  (bind _spherecollision (Variables|Default|GetSphereCollision))
  (Transformation|SetWorldScale3D _spherecollision (Variables|Default|GetScale))
  (Collision|BindEventtoOnComponentBeginOverlap _spherecollision (EventDispatchers|CreateEvent :!event HandleOverlap)))

(fn HandleOverlap
  (params (OverlappedComponent :type Primitive%20Component%20Object%20Reference) (OtherActor :type Actor%20Object%20Reference) (OtherComp :type Primitive%20Component%20Object%20Reference) (OtherBodyIndex :type Integer) (bFromSweep :type Boolean) (SweepResult :type Hit%20Result%20Structure%20%28by%20ref%29))
  (Game|Damage|ApplyDamage OtherActor (Variables|Default|GetDamage) (Variables|Default|GetOwnerController) self)
  (return))