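; Base enemy character that chases the player on entering its sphere collider and gives up once it strays beyond a range from its spawn anchor.
; Chase and stop events swap walk speed and Behavior Trees (chase or wander) and set or clear the TargetActor blackboard key.
; Damage feeds a health component with debug prints.
; Tick polls health to ragdoll the mesh at zero, then disables itself after a delay.
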(event OnComponentBeginOverlap(SphereCollider)
  (params (OverlappedComponent :type Primitive%20Component%20Object%20Reference) (OtherActor :type Actor%20Object%20Reference) (OtherComp :type Primitive%20Component%20Object%20Reference) (OtherBodyIndex :type Integer) (bFromSweep :type Boolean) (SweepResult :type Hit%20Result%20Structure%20%28by%20ref%29))
  (if (== OtherActor (Game|GetPlayerCharacter 0))
    (CallFunction|StartChase)
    (AI|Components|Blackboard|SetValueasObject (AI|GetBlackboard (AI|GetAIController self)) (Utilities|Name|MakeLiteralName "TargetActor") OtherActor)))

(event Custom|StartChase
  (Variables|Default|SetIsChasing true)
  (Variables|/Script/Engine.CharacterMovementComponent|SetMaxWalkSpeed (Variables|Character|GetCharacterMovement) (Variables|Default|GetChaseSpeed))
  (AI|RunBehaviorTree (AI|GetAIController self) "/Game/Enemies/Behavior/BT_BaseEnemy_Chase.BT_BaseEnemy_Chase"))

(event Custom|StopChase
  (Variables|Default|SetIsChasing false)
  (Variables|/Script/Engine.CharacterMovementComponent|SetMaxWalkSpeed (Variables|Character|GetCharacterMovement) (Variables|Default|GetWalkSpeed))
  (AI|RunBehaviorTree (AI|GetAIController self) "/Game/Enemies/Behavior/BT_BaseEnemy_Wander.BT_BaseEnemy_Wander")
  (AI|Components|Blackboard|ClearValue (AI|GetBlackboard (AI|GetAIController self)) (Utilities|Name|MakeLiteralName "TargetActor")))

(event EventBeginPlay
  (Variables|Default|SetAnchor (Transformation|GetActorLocation))
  (Variables|/Script/Engine.CharacterMovementComponent|SetMaxWalkSpeed (Variables|Character|GetCharacterMovement) (Variables|Default|GetWalkSpeed))
  (Variables|/Game/TopDown/Blueprints/Utility/AC_HealthComponent.AC_HealthComponent_C|SetMaxHealth (Variables|Default|GetAC_HealthComponent) 1e+01))

(event Collision|EventActorBeginOverlap
  (params (OtherActor :type Actor%20Object%20Reference)))

(event Game|Damage|EventAnyDamage
  (params (Damage :type Float%20%28single-precision%29) (DamageType :type Damage%20Type%20Object%20Reference) (InstigatedBy :type Controller%20Object%20Reference) (DamageCauser :type Actor%20Object%20Reference))
  (bind _ac_healthcomponent (Variables|Default|GetAC_HealthComponent))
  (Development|PrintString (Utilities|String|ToString(Float) Damage))
  (Development|PrintString (Utilities|String|ToString(Float) (Variables|/Game/TopDown/Blueprints/Utility/AC_HealthComponent.AC_HealthComponent_C|GetCurrentHealth _ac_healthcomponent)))
  (Default|HandleDamage _ac_healthcomponent self Damage))

(event EventTick
  (params (DeltaSeconds :type Float%20%28single-precision%29))
  (bind _mesh (Variables|Character|GetMesh))
  (if (<= (Variables|/Game/TopDown/Blueprints/Utility/AC_HealthComponent.AC_HealthComponent_C|GetCurrentHealth (Variables|Default|GetAC_HealthComponent)) 0.0)
    ;[1 1 1] Ragdoll Effect
    (Physics|SetSimulatePhysics _mesh true)
    (Class|SkeletalMeshComponent|SetPhysicsBlendWeight _mesh 1.0)
    (Collision|SetCollisionEnabled _mesh "QueryAndPhysics")
    (Utilities|FlowControl|Delay 1.0)
    (Actor|Tick|SetActorTickEnabled false)
    (elif (Variables|Default|GetIsChasing)
      (if (> (Math|Vector|Distance(Vector) (Variables|Default|GetAnchor) (Transformation|GetActorLocation)) (Variables|Default|GetRange))
        (CallFunction|StopChase)))))

(fn ConstructionScript)