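; Wave spawner that spawns random enemy classes at spawn points taken from BP_LevelGenerator's SpawnList.
; Tick starts spawning when no BP_BaseEnemy actors remain, using a Delay to release one AI pawn running BT_Final about every second.
; When the count runs out, NextWave notifies BP_TopDownCharacter and sizes the next batch by wave number.
; Spawn location and rotation come from separate random picks, and spawning ignores collision.
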(event Custom|PopulateSpawnLocations
  ;[0 1 0.08394] Set Spawn Locations Array
  (bind _returnvalue (Actor|GetActorOfClass "/Game/PGC_Level/BP_LevelGenerator.BP_LevelGenerator_C"))
  (Variables|Default|SetSpawnLocations (Variables|/Game/PGC_Level/BP_LevelGenerator.BP_LevelGenerator_C|GetSpawnList _returnvalue)))

(event EventBeginPlay
  ;[1 1 1] Begin Play
  (|CallParentFunction)
  (CallFunction|PopulateSpawnLocations))

(event EventTick
  (params (DeltaSeconds :type Float%20%28single-precision%29))
  ;[1 1 1] On Tick
  (|CallParentFunction 0.0)
  (if (Variables|Default|GetCurrentlySpawning)
    (if (> (Variables|Default|GetNumToSpawn) 0) :!label _label
      (Utilities|FlowControl|Delay 1.0)
      (CallFunction|SpawnEnemies)
      (Variables|Default|SetCurrentlySpawning true)
      (else
        (CallFunction|NextWave)
        (Variables|Default|SetCurrentlySpawning false)))
    (else
      (bind _enemiesremain (CallFunction|CheckEnemies))
      (if (not _enemiesremain)
        (goto _label)))))

(fn ConstructionScript)

(fn SpawnEnemies
  (bind _spawnlocations (Variables|Default|GetSpawnLocations))
  (bind _outitem (Utilities|Array|Random _spawnlocations))
  (bind _returnvalue (Transformation|GetWorldTransform _outitem))
  (Variables|Default|SetNumToSpawn (- (Variables|Default|GetNumToSpawn) 1))
  (AI|SpawnAIFromClass (.OutItem (Utilities|Array|Random (Variables|Default|GetEnemyClasses))) "/Game/Enemies/Behavior/BT_Final.BT_Final" (.location _returnvalue) (.rotation _returnvalue) true 0))

(fn CheckEnemies
  (bind _outactors (Actor|GetAllActorsOfClass "/Game/Enemies/BP_BaseEnemy.BP_BaseEnemy_C"))
  (if (Utilities|Array|IsValidIndex _outactors)
    (return true)
    (else
      (return false))))

(fn NextWave
  (Variables|Default|SetWaveCount (+ (Variables|Default|GetWaveCount) 1))
  (bind _returnvalue (Actor|GetActorOfClass "/Game/TopDown/Blueprints/BP_TopDownCharacter.BP_TopDownCharacter_C"))
  (Default|IncreaseWaveCount _returnvalue)
  (Variables|Default|SetNumToSpawn (* (+ (Variables|Default|GetNumToSpawn) 10) (Variables|Default|GetWaveCount))))